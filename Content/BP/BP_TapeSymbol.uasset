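; BP_TapeSymbol is an actor that displays one tape symbol through a widget component.
; The SetSymbol event converts the new symbol to text and writes it into the component's UWSymbol widget.
; GetSymbol reads that text back as a string, so the widget itself holds the symbol state and no separate variable is used.
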(event `self.SetSymbol`
  (params (NewSymbol :type String))
  (`UWSymbol.SetText` (cast `UWSymbol` (`WidgetComponent.GetUserWidgetObject` (`self.Widget`)) :!pure true) (`KismetTextLibrary.Conv_StringToText` NewSymbol)))

(fn `GetSymbol`
  (returns (ReturnValue :type String))
  (return (`KismetTextLibrary.Conv_TextToString` (`UWSymbol.GetText` (cast `UWSymbol` (`WidgetComponent.GetUserWidgetObject` (`self.Widget`)) :!pure true)))))

(fn `UserConstructionScript`)