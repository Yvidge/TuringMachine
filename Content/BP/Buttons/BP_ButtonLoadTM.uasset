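; BP_ButtonLoadTM is a button Blueprint that loads a user-chosen CSV file into the level's BP_TMManager.
; On press, it opens a single-file dialog at the project directory, then sets the first found manager's FilePath and calls ParseDataFromFile.
; It then prints the content directory, project file path and project directory on screen as debug output, whether or not a file was picked.
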(event `self.OnButtonPressed`
  (params (Actor :type "Actor Object Reference") (Key :type "Key Structure"))
  (bind _returnvalue (`KismetSystemLibrary.GetProjectDirectory`))
  (`|ExecutionSequence`
    (:`then_0`
      (bind (_outfilenames _returnvalue_2) (`EFDFunctionLibrary.OpenFileDialog` "BEBRaA" _returnvalue "" ".csv" "Single"))
      (if _returnvalue_2
        (bind _outactors (`GameplayStatics.GetAllActorsOfClass` "/Game/BP/BP_TMManager.BP_TMManager_C"))
        (bind _output (`|GetArrayItem` _outactors))
        (set `TMManager.FilePath` (`|GetArrayItem` _outfilenames) _output)
        (`TMManager.ParseDataFromFile` _output)))
    (:`then_1`
      (`KismetSystemLibrary.PrintString` (`KismetStringLibrary.Concat_StrStr` "Content D :" (`KismetSystemLibrary.GetProjectContentDirectory`)) true true (struct :`R` 1.0 :`G` 0.301269 :`A` 1.0) 20.0)
      (`KismetSystemLibrary.PrintString` (`KismetStringLibrary.Concat_StrStr` "File Path :" (`BlueprintPathsLibrary.GetProjectFilePath`)) true true (struct :`R` 1.0 :`G` 0.489632 :`A` 1.0) 20.0)
      (`KismetSystemLibrary.PrintString` (`KismetStringLibrary.Concat_StrStr` "Project D :" _returnvalue) true true (struct :`R` 1.0 :`G` 0.377587 :`A` 1.0) 20.0))))

(fn `UserConstructionScript`
  (`parent.UserConstructionScript`))