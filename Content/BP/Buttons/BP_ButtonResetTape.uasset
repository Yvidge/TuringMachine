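; BP_ButtonResetTape is a button Blueprint that resets the tape through the BP_TMManager when pressed.
; Its OnButtonPressed event finds all BP_TMManager actors, calls ResetTape on the first one, and prints a "Tape Reseted" debug message.
; The default BeginPlay, overlap and Tick events are disabled, and the construction script only calls its parent.
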(event `self.OnButtonPressed`
  (params (Actor :type "Actor Object Reference") (Key :type "Key Structure"))
  (bind _outactors (`GameplayStatics.GetAllActorsOfClass` "/Game/BP/BP_TMManager.BP_TMManager_C"))
  (`TMManager.ResetTape` (`|GetArrayItem` _outactors))
  (`KismetSystemLibrary.PrintString` "Tape Reseted" true true (struct :`R` 1.0 :`G` 0.048789 :`A` 1.0)))

(fn `UserConstructionScript`
  (`parent.UserConstructionScript`))