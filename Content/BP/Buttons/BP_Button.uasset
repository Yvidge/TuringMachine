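; BP_Button is a pressable button actor with an animated press and an empty OnButtonPressed event.
; PlayPressedAnim runs ClickTimeline at PlayRate, driving the relative Z of ButtonCube scaled by PressDepth.
; A Gate closes as soon as the animation starts and reopens when it finishes, blocking retriggers, while Active is false during the animation.
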(event `self.OnButtonPressed`
  (params (Actor :type "Actor Object Reference") (Key :type "Key Structure")))

(event `self.PlayPressedAnim`
  (`TimelineComponent.SetPlayRate` (`self.ClickTimeline`) (`self.PlayRate`))
  (`|ExecutionSequence`
    (:`then_0`
      (`/Engine/EditorBlueprintResources/StandardMacros.Gate` false :!label _label
        (:`Exit`
          (set `self.bActive` false)
          (bind (_direction _z) (`Timeline|ClickTimeline` :!via `PlayFromStart`)
            (:`Update`
              (`SceneComponent.K2_SetRelativeLocation` (`self.Button_Cube`) (`KismetMathLibrary.MakeVector` 0.0 0.0 (* _z (`self.PressDepth`))) false false))
            (:`Finished`
              (set `self.bActive` true)
              (goto _label :!via `Open`))))))
    (:`then_1`
      (goto _label :!via `Close`))))

(fn `UserConstructionScript`)