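; A button that, when pressed, moves the first player's pawn to the location of a target actor.
; On press it records the pawn's start location and plays a timeline from the start, with play rate set by a speed multiplier.
; Each timeline update lerps the pawn from that start toward the target's current location without sweeping, so collision does not block the move.
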(event `self.OnButtonPressed`
  (params (Actor :type "Actor Object Reference") (Key :type "Key Structure"))
  (`TimelineComponent.SetPlayRate` (`self.Timeline_PawnMovement`) (`self.SpeedMultiplier`))
  (set `self.StartLocation` (`self.K2_GetActorLocation` (`GameplayStatics.GetPlayerPawn` 0)))
  (bind (_direction _alpha) (`Timeline|Timeline_PawnMovement` :!via `PlayFromStart`)
    (:`Update`
      (`self.K2_SetActorLocation` (`GameplayStatics.GetPlayerPawn` 0) (`KismetMathLibrary.VLerp` (`self.StartLocation`) (`self.K2_GetActorLocation` (`self.ActorToTakeLocation`)) _alpha) false false))))

(fn `UserConstructionScript`
  (`parent.UserConstructionScript`))