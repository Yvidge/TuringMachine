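; BP_Tape is a tape with a read/write head, apparently for a Turing-machine-style display, that animates tape shifts and write strokes.
; MoveTape slides SymbolsAnchor one HorizontalSize left, right or not at all based on the Move value, using a timeline with sharp ease-in-out interpolation.
; PlayHeadAnim runs a separate timeline that offsets the Head vertically in world space, scaled by HeadAnimDepth.
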(event `self.MoveTape`
  (params (Move :type "EMoveReaction Enum" :default "L"))
  (bind _relativelocation_x (`KismetMathLibrary.BreakVector` (`SceneComponent.RelativeLocation` (`self.SymbolsAnchor`))))
  (`TimelineComponent.SetPlayRate` (`self.MoveTimeline`) (`self.MovePlayRate`))
  (bind _output_get (set `self.Relative Location X` _relativelocation_x))
  (bind (_direction _xoffset) (`Timeline|MoveTimeline` :!via `PlayFromStart`)
    (:`Update`
      (`SceneComponent.K2_SetRelativeLocation` (`self.SymbolsAnchor`) (`KismetMathLibrary.MakeVector` (`KismetMathLibrary.FInterpEaseInOut` _output_get (+ _output_get (* (`self.HorizontalSize`) (select `EMoveReaction` Move :`L` 1.0 :`R` -1.0 :`N` 0.0))) _xoffset 20.0)) false false))))

(event `self.PlayHeadAnim`
  (bind (_headworldloc_x _headworldloc_y _headworldloc_z) (`KismetMathLibrary.BreakVector` (`self.HeadWorldLoc`)))
  (set `self.HeadWorldLoc` (`SceneComponent.K2_GetComponentLocation` (`self.Head`)))
  (`TimelineComponent.SetPlayRate` (`self.WritingTimeline`) 4.0)
  (bind (_direction _coord) (`Timeline|WritingTimeline` :!via `PlayFromStart`)
    (:`Update`
      (`SceneComponent.K2_SetWorldLocation` (`self.Head`) (`KismetMathLibrary.MakeVector` _headworldloc_x _headworldloc_y (+ (* _coord (`self.HeadAnimDepth`)) _headworldloc_z)) false false))))

(fn `UserConstructionScript`)