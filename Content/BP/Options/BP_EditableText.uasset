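; BP_EditableText is a base Blueprint for an editable text option, driving a WBP_EditableText hosted in its widget component.
; Init, run at construction and BeginPlay, sets the widget's property name and value and caches the first BP_TMManager.
; Text changes bound at BeginPlay route to SetPropertyValue.
; The getter returns a placeholder and the setter is empty, apparently hooks for child Blueprints to override.
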(event `self.ReceiveBeginPlay`
  (`self.Init`)
  (add `/Game/Widgets/WBP_EditableText.OnTextChanged` (`self.EditableTextWidget`) (delegate `OnTextChanged_Event_0`)))

(event `OnTextChanged_Event_0`
  (params (NewValue :type Text))
  (`self.SetPropertyValue` NewValue))

(fn `GetPropertyValue`
  (returns (Value :type Text))
  (return "Value"))

(fn `Init`
  (bind _aswbp_editable_text (cast `/Game/Widgets/WBP_EditableText` (`WidgetComponent.GetWidget` (`self.Widget`))))
  (bind _output_get (set `self.EditableTextWidget` _aswbp_editable_text))
  (`/Game/Widgets/WBP_EditableText.SetPropertyName` _output_get (`self.PropertyName`))
  (bind _outactors (`GameplayStatics.GetAllActorsOfClass` "/Game/BP/BP_TMManager.BP_TMManager_C"))
  (set `self.Manager` (`|GetArrayItem` _outactors))
  (`/Game/Widgets/WBP_EditableText.Set Value` (`self.EditableTextWidget`) (`self.GetPropertyValue`)))

(fn `SetPropertyValue`
  (params (NewValue :type Text)))

(fn `UserConstructionScript`
  (`self.Init`))